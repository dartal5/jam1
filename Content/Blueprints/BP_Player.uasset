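; BP_Player is the playable 2D side-scroller character, using Enhanced Input to run along the Y axis and jump.
; BeginPlay registers the input mapping context on the local player's subsystem.
; Each tick selects a Fall, Running or Idle flipbook from movement state.
; It also snaps controller yaw to the sign of the last Y input so the character faces its travel direction.
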(event `self.ReceiveBeginPlay`
  (bind _asplayer_controller (cast `PlayerController` (`self.GetController`)))
  (bind _returnvalue (pcsubsystem `EnhancedInputLocalPlayerSubsystem` _asplayer_controller))
  (`/Engine/EditorBlueprintResources/StandardMacros.IsValid` _returnvalue
    (:`Is Valid`
      (`EnhancedInputSubsystemInterface.AddMappingContext` _returnvalue "/Game/Input/MainInputContext.MainInputContext" 0 (struct)))))

(event `EnhancedInput|/Game/Input/Actions/IA_Move`
  (params (ActionValue :type "Float (double-precision)") (ElapsedSeconds :type "Float (double-precision)") (TriggeredSeconds :type "Float (double-precision)") (InputAction :type "InputAction Object Reference" :default "/Game/Input/Actions/IA_Move.IA_Move"))
  (:`Triggered`
    (`self.AddMovementInput` (0.0 1.0 0.0) ActionValue)))

(event `EnhancedInput|/Game/Input/Actions/IA_Jump`
  (params (ActionValue :type Boolean) (ElapsedSeconds :type "Float (double-precision)") (TriggeredSeconds :type "Float (double-precision)") (InputAction :type "InputAction Object Reference" :default "/Game/Input/Actions/IA_Jump.IA_Jump"))
  (:`Triggered`
    (`self.Jump`)))

(event `self.ReceiveTick`
  (params (DeltaSeconds :type "Float (single-precision)"))
  (`self.UpdateAnimation`)
  (`self.UpdateControlRotation`))

(event `UpdateAnimation`
  (`PaperFlipbookComponent.SetFlipbook` (`self.Sprite`) (select `bool` (`NavMovementComponent.IsFalling` (`self.CharacterMovement`)) :`false` (select `bool` (!= (`KismetMathLibrary.VSize` (`MovementComponent.Velocity` (`self.CharacterMovement`))) 0.0) :`false` "/Game/Levels/Character/FlipBooks/Idle.Idle" :`true` "/Game/Levels/Character/FlipBooks/Running.Running" :!type "PaperFlipbook Object Reference") :`true` "/Game/Levels/Character/FlipBooks/Fall.Fall")))

(event `UpdateControlRotation`
  (`/Engine/EditorBlueprintResources/StandardMacros.IsValid` (`self.GetController`)
    (:`Is Valid`
      (`/Engine/EditorBlueprintResources/StandardMacros.CompareFloat` (.y (`PawnMovementComponent.GetLastInputVector` (`self.CharacterMovement`)))
        (:`>`
          (`Controller.SetControlRotation` (`self.GetController`) (`KismetMathLibrary.MakeRotator` 0.0 0.0 90.0)))
        (:`<`
          (`Controller.SetControlRotation` (`self.GetController`) (`KismetMathLibrary.MakeRotator` 0.0 0.0 -90.0)))))))

(fn `UserConstructionScript`)